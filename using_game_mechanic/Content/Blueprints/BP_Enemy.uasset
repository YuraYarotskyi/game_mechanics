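; BP_Enemy is an enemy actor that patrols back and forth along a horizontal diagonal and damages any actor that overlaps it.
; A looping Timeline adds its track value, scaled by K, to the current X and Y on each update, and K flips sign on each finish to reverse direction.
; Yaw is derived from the Y position plus that same step, so rotation follows location rather than heading.
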(event `self.ReceiveBeginPlay`
  (bind (_returnvalue_x _returnvalue_y _returnvalue_z) (`KismetMathLibrary.BreakVector` (`self.K2_GetActorLocation`)))
  (bind _k (`self.K`))
  (bind (_direction _newtrack_0) (`Timeline|Timeline` :!label _label)
    (:`Update`
      (bind _returnvalue (* _newtrack_0 _k))
      (bind _returnvalue_2 (+ _returnvalue_y _returnvalue))
      (`self.K2_SetActorLocation` (`KismetMathLibrary.MakeVector` (+ _returnvalue_x _returnvalue) _returnvalue_2 _returnvalue_z))
      (`self.K2_SetActorRotation` (`KismetMathLibrary.MakeRotator` 0.0 0.0 _returnvalue_2)))
    (:`Finished`
      (set `self.K` (* _k -1.0))
      (goto _label :!via `PlayFromStart`))))

(event `self.ReceiveActorBeginOverlap`
  (params (OtherActor :type "Actor Object Reference"))
  (`GameplayStatics.ApplyDamage` OtherActor 10.0 null self))

(fn `UserConstructionScript`)