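; AC_Health is a component that tracks its owner's health and reports changes through the Gameplay Message Subsystem.
; On BeginPlay it fills Health to MaxHealth and binds to the owner's OnTakeAnyDamage.
; Each hit subtracts damage, broadcasts Player.death when Health is no longer above zero, and always broadcasts Player.health with the current value and bar ratio.
; Health is not clamped, so further hits after death broadcast death again.
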(event `self.ReceiveBeginPlay`
  (set `self.health` (`self.max_health`))
  (add `Actor.OnTakeAnyDamage` (`self.GetOwner`) (delegate `Damage`)))

(event `Damage`
  (params (DamagedActor :type "Actor Object Reference") (Damage :type "Float (single-precision)") (DamageType :type "DamageType Object Reference") (InstigatedBy :type "Controller Object Reference") (DamageCauser :type "Actor Object Reference"))
  (bind _returnvalue (subsystem `GameplayMessageSubsystem`))
  (bind _output_get (set `self.health` (- (`self.health`) Damage)))
  (if (not (> _output_get 0.0))
    (`GameplayMessageSubsystem.K2_BroadcastMessage` _returnvalue (struct :`TagName` "player.death") (make `/Game/Blueprints/BS_Empty` false)))
  (`GameplayMessageSubsystem.K2_BroadcastMessage` _returnvalue (struct :`TagName` "player.health") (make `/Game/Blueprints/BS_Health` _output_get (/ (`self.health`) (`self.max_health`)))))